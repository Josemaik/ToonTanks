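; Game mode for Toon Tanks that puts the start, end-game and score screens on the viewport.
; StartGame, GameOver and ShowPuntuation events each create their widget and add it to the viewport.
; GameOver sets the win or lose text from WonGame, and on a loss also reveals the Respawn widget element and empties the tank's life bar.
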(event EventBeginPlay)

(event EventTick
  (params (DeltaSeconds :type Float%20%28single-precision%29)))

(event EventStartGame
  (bind _returnvalue (UserInterface|CreateWidget "/Game/Blueprints/Widgets/WBP_StartGameWidget.WBP_StartGameWidget_C"))
  (UserInterface|Viewport|AddtoViewport _returnvalue 0))

(event EventGameOver
  (params (bWonGame :type Boolean))
  (bind _returnvalue (UserInterface|CreateWidget "/Game/Blueprints/Widgets/WBP_EndGameWidget1.WBP_EndGameWidget1_C"))
  (UserInterface|Viewport|AddtoViewport _returnvalue 0)
  (Rendering|Components|TextRender|SetText (Variables|/Game/Blueprints/Widgets/WBP_EndGameWidget1.WBP_EndGameWidget1_C|GetDisplayText _returnvalue) (Utilities|Text|ToText(String) (Utilities|String|SelectString "You win the Game!" "You lose the Game!" bWonGame)))
  (if (not bWonGame)
    (Widget|SetVisibility (Variables|/Game/Blueprints/Widgets/WBP_EndGameWidget1.WBP_EndGameWidget1_C|GetRespawn _returnvalue) "Visible")
    (Progress|SetPercent (Variables|/Game/Blueprints/Widgets/WBP_lifeBarTank.WBP_lifeBarTank_C|GetProgressBar_114 (Variables|Default|GetRefWBLifeBarTank)) 0.0)))

(event EventShowPuntuation
  (bind _returnvalue (UserInterface|CreateWidget "/Game/Blueprints/Widgets/WBP_Puntuation.WBP_Puntuation_C"))
  (UserInterface|Viewport|AddtoViewport _returnvalue 0))

(fn ConstructionScript)